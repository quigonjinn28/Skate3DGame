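; BP_JumpableObject is an obstacle actor that awards score when the skater jumps over it.
; Overlap events, with a detection sphere sized on BeginPlay, store the overlapping BP_SkaterCharacter.
; While one is stored, Tick box-traces upward from the mesh, using its scaled bounds and debug drawing, to flag a jump when the skater is hit.
; Ending overlap calls AddScore on the game mode if flagged, then clears the state.
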(event `self.ReceiveBeginPlay`
  (`SphereComponent.SetSphereRadius` (`self.Sphere`) (`self.DetectionRadius`) true))

(event `self.ReceiveActorBeginOverlap`
  (params (OtherActor :type "Actor Object Reference"))
  (bind _asbp_skater_character (cast `/Game/Blueprints/Skater/BP_SkaterCharacter` OtherActor))
  (set `self. SkateRef` _asbp_skater_character))

(event `self.ReceiveActorEndOverlap`
  (params (OtherActor :type "Actor Object Reference"))
  (if (and (== OtherActor (`self. SkateRef`)) (`self.HasJumped`))
    (bind _asbp_skater_game_mode (cast `/Game/Blueprints/GameMode/BP_SkaterGameMode` (`GameplayStatics.GetGameMode`)))
    (`/Game/Blueprints/GameMode/BP_SkaterGameMode.AddScore` _asbp_skater_game_mode))
  (set `self. SkateRef` null)
  (set `self.HasJumped` false))

(event `self.ReceiveTick`
  (params (DeltaSeconds :type "Float (single-precision)"))
  (bind _returnvalue (`SceneComponent.K2_GetComponentLocation` (`self.Mesh`)))
  (if (`KismetSystemLibrary.IsValid` (`self. SkateRef`))
    (bind (_outhit _returnvalue_2) (`KismetSystemLibrary.BoxTraceSingle` :`Start` _returnvalue :`End` (+ _returnvalue (`KismetMathLibrary.MakeVector` 0.0 0.0 (`self.JumpDetectionHeight`))) :`HalfSize` (* (`.BoxExtent` (`KismetSystemLibrary.GetComponentBounds` (`self.Mesh`))) 0.9) :`TraceChannel` "TraceTypeQuery1" :`DrawDebugType` "ForOneFrame"))
    (if (and _returnvalue_2 (== (`.HitActor` (`GameplayStatics.BreakHitResult` _outhit)) (`self. SkateRef`)))
      (set `self.HasJumped` true))))

(fn `UserConstructionScript`)